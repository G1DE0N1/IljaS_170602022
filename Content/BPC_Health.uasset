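; BPC_Health is a health component that tracks the current Health of its owner against a MaxHealth.
; It refills Health to MaxHealth on BeginPlay through Recovery.
; AddHealth caps healing at MaxHealth and Damage floors at zero, while GetHealth and IsDead expose the current value and whether it has run out.
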(event EventBeginPlay
  (CallFunction|Recovery))

(event EventTick
  (params (DeltaSeconds :type Float%20%28single-precision%29)))

(fn GetHealth
  (return (Variables|Default|GetHealth)))

(fn IsDead
  (return (<= (Variables|Default|GetHealth) 0.0)))

(fn AddHealth
  (params (Add :type Float%20%28single-precision%29))
  (Variables|Default|SetHealth (Math|Float|Min(Float) (+ Add (Variables|Default|GetHealth)) (Variables|Default|GetMaxHealth)))
  (return))

(fn Damage
  (params (Damage :type Float%20%28single-precision%29))
  (Variables|Default|SetHealth (Math|Float|Max(Float) (- (Variables|Default|GetHealth) Damage) 0.0))
  (return))

(fn Recovery
  (Variables|Default|SetHealth (Variables|Default|GetMaxHealth))
  (return))